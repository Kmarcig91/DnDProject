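; BP_Tile3 is an interactive tile that reacts to mouse hover and click through a dynamic material on its top mesh.
; Its construction script caches the default emission and, for tiles above world zero, stacks body meshes beneath the top according to height.
; Hover sets a hand cursor and plays an emission flash timeline, then polls with a delay loop and debug prints until the cursor leaves, restoring emission.
; Clicking turns the top bright glowing green.
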(event OnBeginCursorOver(TileTop)
  (params (TouchedComponent :type Primitive%20Component%20Object%20Reference))
  (bind _asbp_player_controller (Utilities|Casting|CastToBP_PlayerController (Game|GetPlayerController 0)))
  (Variables|/Script/Engine.PlayerController|SetCurrentMouseCursor _asbp_player_controller "Hand")
  (Variables|Default|SetisCursorOver true)
  (Development|PrintString "Hello, World!")
  (bind _flashalpha (Timeline|TileFlashLerp PlayFromStart)
    (:Update
      (Rendering|Material|SetScalarParameterValue (Variables|Default|GetTileTopMID) "TileEmission" (Math|Float|Lerp (Variables|Default|GetTileEmissionDefault) 5e+01 _flashalpha) :!class /Script/Engine.MaterialInstanceDynamic))
    (:Finished
      (if (Variables|Default|GetisCursorOver) :!label _label
        (Utilities|FlowControl|Delay 0.5)
        (Development|PrintString "Standing Still!" true true "(R=0.000000,G=0.370000,B=0.086191,A=1.000000)")
        (goto _label)
        (else
          (Development|PrintString "Goodbye, World!")
          (Rendering|Material|SetScalarParameterValue (Variables|Default|GetTileTopMID) "TileEmission" (Variables|Default|GetTileEmissionDefault) :!class /Script/Engine.MaterialInstanceDynamic))))))

(event OnEndCursorOver(TileTop)
  (params (TouchedComponent :type Primitive%20Component%20Object%20Reference))
  (bind _asbp_player_controller (Utilities|Casting|CastToBP_PlayerController (Game|GetPlayerController 0)))
  (Variables|/Script/Engine.PlayerController|SetCurrentMouseCursor _asbp_player_controller "Default")
  (Variables|Default|SetisCursorOver false))

(event OnClicked(TileTop)
  (params (TouchedComponent :type Primitive%20Component%20Object%20Reference) (ButtonPressed :type Key%20Structure :default "AnyKey"))
  (bind _tiletopmid (Variables|Default|GetTileTopMID))
  (Rendering|Material|SetScalarParameterValue _tiletopmid "TileEmission" 1e+03 :!class /Script/Engine.MaterialInstanceDynamic)
  (Rendering|Material|SetVectorParameterValue _tiletopmid "TileTopColor" "(R=0.000000,G=0.880000,B=0.005828,A=1.000000)" :!class /Script/Engine.MaterialInstanceDynamic))

(event EventBeginPlay)

(event Collision|EventActorBeginOverlap
  (params (OtherActor :type Actor%20Object%20Reference)))

(event EventTick
  (params (DeltaSeconds :type Float%20%28single-precision%29)))

(fn ConstructionScript
  (bind _tiletop (Variables|Default|GetTileTop))
  (bind _returnvalue (Transformation|GetWorldLocation _tiletop))
  (bind _returnvalue_2 (Rendering|Material|CreateDynamicMaterialInstance (Variables|Default|GetTileTop) 0 0 :!class /Script/Engine.PrimitiveComponent))
  (bind _output_get (Variables|Default|SetTileTopMID _returnvalue_2))
  (bind _returnvalue_3 (Rendering|Material|GetScalarParameterValue _output_get "TileEmission" :!class /Script/Engine.MaterialInstanceDynamic))
  (Variables|Default|SetTileEmissionDefault _returnvalue_3)
  (if (> (.z _returnvalue) 0.0)
    (bind _returnvalue_4 (AddComponent|AddStaticMeshComponent false))
    (Rendering|Material|SetMaterial _returnvalue_4 0 (Variables|Default|GetBodyMaterial))
    (for _index (range 0 (- (.ReturnValue (Math|Float|Division(WholeandRemainder) (.z _returnvalue) 2e+01)) 1))
      (bind _returnvalue_5 (AddComponent|AddStaticMeshComponent false))
      (Rendering|Material|SetMaterial _returnvalue_5 0 (Variables|Default|GetBodyMaterial))
      (Transformation|SetRelativeLocation _returnvalue_5 (Math|Vector|MakeVector 0.0 0.0 (Math|Conversions|ToFloat(Integer) (- (* _index -20) 40))) false false))))